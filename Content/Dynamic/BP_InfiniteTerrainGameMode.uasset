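; Game mode for an infinite terrain game that chains BP_Tile actors together and keeps a score.
; On BeginPlay it populates a bounds volume pool, then spawns an initial run of tiles.
; SpawnTile passes the NavMeshPool to each new tile and stores its attach location as the next spawn transform.
; TileConquered increments the score.
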(event `self.ReceiveBeginPlay`
  (`self.PopulateBoundsVolumePool`)
  (for _ (range 4)
    (`self.Spawn Tile`)))

(fn `Spawn Tile`
  (bind _returnvalue (`|SpawnActorFromClass` "/Game/Dynamic/Terrain/BP_Tile.BP_Tile_C" (`self.nextTileTransform`) "Undefined" "OverrideRootScale"))
  (`Tile.SetPool` _returnvalue (`self.NavMeshPool`))
  (bind _attach_transform (`/Game/Dynamic/Terrain/BP_Tile.Get Attach Location` _returnvalue))
  (set `self.nextTileTransform` _attach_transform))

(fn `Tile Conquered`
  (bind _result (`/Engine/EditorBlueprintResources/StandardMacros.IncrementInt` (`self.Score`))
    (:`  `
      (set `self.Score` _result))))

(fn `UserConstructionScript`)